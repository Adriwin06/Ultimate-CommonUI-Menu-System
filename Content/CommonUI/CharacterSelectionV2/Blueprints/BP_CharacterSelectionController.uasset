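; Controller for the CommonUI character selection screen that opens the selection menu and drives switching between characters.
; On begin play it creates a container widget, adds it to the viewport and pushes the character selection menu onto it.
; SwitchCharacter fires event dispatchers to play a sequence forward or in reverse, ignoring requests while one is playing.
; Pausing the sequence broadcasts its own event and clears that playing flag.
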(event `self.ReceiveBeginPlay`
  (`parent.ReceiveBeginPlay`)
  (bind _returnvalue (`|CreateWidget` "/Game/CommonUI/Foundation/Widgets/BPW_Container.BPW_Container_C"))
  (`UserWidget.AddToViewport` _returnvalue 0)
  (`/Game/CommonUI/Foundation/Widgets/BPW_Container.PushMenu` _returnvalue "/Game/CommonUI/CharacterSelectionV2/Widgets/UI_CharacterSelectionV2.UI_CharacterSelectionV2_C"))

(event `PlaySequence`
  (`self.PlaySequenceEvent`))

(event `PlaySequenceInReverse`
  (`self.PlaySequenceInReverseEvent`))

(event `PauseSequence`
  (`self.PauseSequenceEvent`)
  (set `self.bIsSequencePlaying` false))

(fn `SwitchCharacter`
  (params (`bDecreasing?` :type Boolean))
  (if (not (`self.bIsSequencePlaying`))
    (if `bDecreasing?`
      (`self.PlaySequenceInReverse`)
      (else
        (`self.PlaySequence`)))
    (set `self.bIsSequencePlaying` true)))

(fn `UserConstructionScript`
  (`parent.UserConstructionScript`))