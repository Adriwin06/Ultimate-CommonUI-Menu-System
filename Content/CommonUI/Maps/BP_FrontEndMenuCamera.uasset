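; Front-end menu camera actor that drifts its camera using the CameraMovement timeline, started on BeginPlay.
; Each update adds the track values to the camera's current world location, with the Y track driving world X and X driving Y, and leaves rotation unset.
; On finish it calls ContinueMoving to play again; custom events offer play-from-start and reverse-from-end.
; StartLocation is saved but never read here.
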(event `self.ReceiveBeginPlay`
  (set `self.StartLocation` (`SceneComponent.K2_GetComponentToWorld` (`self.CameraComponent`)))
  (`self.ContinueMoving`))

(event `ContinueMoving`
  (bind _returnvalue (`SceneComponent.K2_GetComponentToWorld` (`self.CameraComponent`)))
  (bind (_direction _ycammovement _xcammovement _zcammovement) (`Timeline|CameraMovement` :!label _label)
    (:`Update`
      (`SceneComponent.K2_SetWorldTransform` (`self.CameraComponent`) (`KismetMathLibrary.MakeTransform` (`KismetMathLibrary.MakeVector` (+ _ycammovement (.x (.location _returnvalue))) (+ _xcammovement (.y (.location _returnvalue))) (+ _zcammovement (.z (.location _returnvalue))))) false false))
    (:`Finished`
      (`self.ContinueMoving`))))

(event `MoveFromStart`
  (goto _label :!via `PlayFromStart`))

(event `MoveReverseFromEnd`
  (goto _label :!via `ReverseFromEnd`))

(fn `UserConstructionScript`)