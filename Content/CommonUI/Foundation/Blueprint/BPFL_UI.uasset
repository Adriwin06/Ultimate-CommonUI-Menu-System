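; Blueprint function library for the CommonUI menus that applies saved user options and handles confirmation prompts.
; ApplyAllUserSettings loads separate save slots for graphics, video and audio, feeding a post-process volume, GameUserSettings, console variables, upscaler plugins (DLSS, FSR3, XeSS, NIS) and a sound mix.
; Non-master volumes are scaled by master volume.
; ShowPrompt pushes button-defined prompts to BPW_Container, and PromptAction switches on PromptID to quit or return to the main menu.
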(fn `ApplyAllUserSettings`
  (`self.ApplyGraphicsSettings` null)
  (`self.ApplyVideoSettings` null)
  (`self.ApplyAudioSettings` null))

(fn `ApplyAudioSettings`
  (locals (MasterVolumeMultiplier :type "Float (double-precision)" :default 1.0) (`Sound Mix Modifier` :type "SoundMix Object Reference" :default "/Script/Engine.SoundMix'/Game/CommonUI/Settings/Sound/VolumeSoundClassMix.VolumeSoundClassMix'"))
  (bind _sound_mix_modifier (`local.Sound Mix Modifier`))
  (bind (_asbp_options_save_game _savegameexist) (`self.LoadSaveGame` "AudioSettingsSaveSlot0"))
  (if _savegameexist
    (`|ExecutionSequence`
      (:`then_0`
        (`|ExecutionSequence`
          (:`then_0`
            (bind (_mastervolume _musicvolume _voicesvolume _ambiencevolume _soundsvolume _uivolume _controllerspeakervolume) (break `/Game/CommonUI/Settings/Data/Struct_AudioSettings` (`/Game/CommonUI/Save/BP_OptionsSaveGame.AllAudioSettings` _asbp_options_save_game)))
            (bind _returnvalue (/ _mastervolume 100.0))
            (`GameplayStatics.SetSoundMixClassOverride` null _sound_mix_modifier "/Game/CommonUI/Settings/Sound/Master.Master" _returnvalue)
            (set `local.MasterVolumeMultiplier` _returnvalue))
          (:`then_1`
            (`GameplayStatics.SetSoundMixClassOverride` null _sound_mix_modifier "/Game/CommonUI/Settings/Sound/Music.Music" (* (/ _musicvolume 100.0) (`local.MasterVolumeMultiplier`))))
          (:`then_2`
            (`GameplayStatics.SetSoundMixClassOverride` null _sound_mix_modifier "/Game/CommonUI/Settings/Sound/Voice.Voice" (* (/ _voicesvolume 100.0) (`local.MasterVolumeMultiplier`))))
          (:`then_3`
            (`GameplayStatics.SetSoundMixClassOverride` null _sound_mix_modifier "/Game/CommonUI/Settings/Sound/Ambience.Ambience" (* (/ _ambiencevolume 100.0) (`local.MasterVolumeMultiplier`))))
          (:`then_4`
            (`GameplayStatics.SetSoundMixClassOverride` null _sound_mix_modifier "/Game/CommonUI/Settings/Sound/SFX.SFX" (* (/ _soundsvolume 100.0) (`local.MasterVolumeMultiplier`))))
          (:`then_5`
            (`GameplayStatics.SetSoundMixClassOverride` null _sound_mix_modifier "/Game/CommonUI/Settings/Sound/UI.UI" (* (/ _uivolume 100.0) (`local.MasterVolumeMultiplier`))))
          (:`then_6`
            (`GameplayStatics.SetSoundMixClassOverride` null _sound_mix_modifier "/Game/CommonUI/Settings/Sound/ControllerSpeaker.ControllerSpeaker" (* (/ _controllerspeakervolume 100.0) (`local.MasterVolumeMultiplier`))))))
      (:`then_1`
        (`GameplayStatics.PushSoundMixModifier` null (`local.Sound Mix Modifier`))))))

(fn `ApplyGraphicsSettings`
  (locals (AllGraphicsSettings :type "/Game/CommonUI/Settings/Data/Struct_GraphicsSettings Structure"))
  (bind (_asbp_options_save_game _savegameexist) (`self.LoadSaveGame` "OptionsSaveSlot0"))
  (if _savegameexist
    (bind _output_get (set `local.AllGraphicsSettings` (`/Game/CommonUI/Save/BP_OptionsSaveGame.AllGraphicsSettings` _asbp_options_save_game)))
    (bind _returnvalue (`GameplayStatics.GetActorOfClass` null "/Script/Engine.PostProcessVolume"))
    (set `PostProcessVolume.Settings` (`.PostProcessVolumeSettings_31_000FB778430AFFB825DBD386FD87CE05` (break `/Game/CommonUI/Settings/Data/Struct_GraphicsSettings` _output_get)) _returnvalue)))

(fn `ApplyVideoSettings`
  (locals (UI_VideoSettingsRef :type "UserWidget Object Reference") (AllVideoSettings :type "/Game/CommonUI/Settings/Data/Struct_VideoSettings Structure"))
  (bind (_allvideosettings_maxfps _allvideosettings_bvsyncenabled _allvideosettings_reflexoptionid _allvideosettings_aaoptionid _allvideosettings_msaasamplesoptionid _allvideosettings_screenpercentage _allvideosettings_dlssmodeswitcher _allvideosettings_dlssqualityoptionid _allvideosettings_nissharpness _allvideosettings_bdlss_rrenabled _allvideosettings_fsrmodeoptionid _allvideosettings_bfsr3framegenenabled _allvideosettings_fsr3sharpness _allvideosettings_xessmodeoptionid _allvideosettings_nismodeoptionid _allvideosettings_niscustomscreenpercentage _allvideosettings_upscalemodeoptionid _allvideosettings_resolutionoptionid _allvideosettings_windowmodeoptionid) (break `/Game/CommonUI/Settings/Data/Struct_VideoSettings` (`local.AllVideoSettings`)))
  (bind (_asbp_options_save_game _savegameexist) (`self.LoadSaveGame` "VideoSettingsSaveSlot0"))
  (if _savegameexist
    (set `local.AllVideoSettings` (`/Game/CommonUI/Save/BP_OptionsSaveGame.AllVideoSettings` _asbp_options_save_game))
    (`|ExecutionSequence`
      (:`then_0`
        (bind _returnvalue (`GameUserSettings.GetGameUserSettings`))
        (bind _resolutions (`KismetSystemLibrary.GetSupportedFullscreenResolutions`))
        (for (_array_element _array_index) _resolutions
          (if (== _array_index _allvideosettings_resolutionoptionid)
            (`GameUserSettings.SetScreenResolution` _returnvalue _array_element))))
      (:`then_1`
        (bind _returnvalue_2 (`GameUserSettings.GetGameUserSettings`))
        (switch `int` _allvideosettings_windowmodeoptionid
          (:`0`
            (`GameUserSettings.SetFullscreenMode` _returnvalue_2 "Fullscreen"))
          (:`1`
            (`GameUserSettings.SetFullscreenMode` _returnvalue_2 "WindowedFullscreen"))
          (:`2`
            (`GameUserSettings.SetFullscreenMode` _returnvalue_2 "Windowed"))))
      (:`then_2`
        (bind _returnvalue_3 (`GameUserSettings.GetGameUserSettings`))
        (`GameUserSettings.SetFrameRateLimit` _returnvalue_3 _allvideosettings_maxfps)
        (`GameUserSettings.ApplySettings` _returnvalue_3 false))
      (:`then_3`
        (bind _returnvalue_4 (`GameUserSettings.GetGameUserSettings`))
        (`GameUserSettings.SetVSyncEnabled` _returnvalue_4 _allvideosettings_bvsyncenabled)
        (`GameUserSettings.ApplySettings` _returnvalue_4 false))
      (:`then_4`
        (switch `int` _allvideosettings_reflexoptionid
          (:`0`
            (`StreamlineLibraryReflex.SetReflexMode` "Disabled"))
          (:`1`
            (`StreamlineLibraryReflex.SetReflexMode` "Enabled"))
          (:`2`
            (`StreamlineLibraryReflex.SetReflexMode` "EnabledPlusBoost"))))
      (:`then_5`
        (`KismetSystemLibrary.ExecuteConsoleCommand` null (`KismetStringLibrary.BuildString_Int` "" "r.AntiAliasingMethod " _allvideosettings_aaoptionid) null))
      (:`then_6`
        (switch `int` _allvideosettings_msaasamplesoptionid
          (:`0`
            (`KismetSystemLibrary.ExecuteConsoleCommand` null "r.MSAACount 0" null))
          (:`1`
            (`KismetSystemLibrary.ExecuteConsoleCommand` null "r.MSAACount 1" null))
          (:`2`
            (`KismetSystemLibrary.ExecuteConsoleCommand` null "r.MSAACount 2" null))
          (:`3`
            (`KismetSystemLibrary.ExecuteConsoleCommand` null "r.MSAACount 4" null))
          (:`4`
            (`KismetSystemLibrary.ExecuteConsoleCommand` null "r.MSAACount 8" null))))
      (:`then_7`
        (`KismetSystemLibrary.ExecuteConsoleCommand` null (`KismetStringLibrary.BuildString_Double` "" "r.ScreenPercentage " _allvideosettings_screenpercentage) null))
      (:`then_8`
        (switch `int` _allvideosettings_dlssmodeswitcher
          (:`0`
            (`StreamlineLibraryDLSSG.SetDLSSGMode` "Off"))
          (:`1`
            (`StreamlineLibraryDLSSG.SetDLSSGMode` "On"))
          (:`2`
            (`StreamlineLibraryDLSSG.SetDLSSGMode` "Auto"))))
      (:`then_9`
        (if (> _allvideosettings_dlssqualityoptionid 0)
          (switch `int` _allvideosettings_dlssqualityoptionid
            (:`0`
              (`/DLSS/DLSSMacros.Set DLSS/DLAA Mode (no auto)` "Off" false true))
            (:`1`
              (`/DLSS/DLSSMacros.Set DLSS/DLAA Mode (no auto)` "Auto" false true))
            (:`2`
              (`/DLSS/DLSSMacros.Set DLSS/DLAA Mode (no auto)` "DLAA" false true))
            (:`3`
              (`/DLSS/DLSSMacros.Set DLSS/DLAA Mode (no auto)` "UltraQuality" false true))
            (:`4`
              (`/DLSS/DLSSMacros.Set DLSS/DLAA Mode (no auto)` "Quality" false true))
            (:`5`
              (`/DLSS/DLSSMacros.Set DLSS/DLAA Mode (no auto)` "Balanced" false true))
            (:`6`
              (`/DLSS/DLSSMacros.Set DLSS/DLAA Mode (no auto)` "Performance"))
            (:`7`
              (`/DLSS/DLSSMacros.Set DLSS/DLAA Mode (no auto)` "UltraPerformance" false true)))))
      (:`then_10`
        (`NISLibrary.SetNISSharpness` _allvideosettings_nissharpness))
      (:`then_11`
        (`DLSSLibrary.EnableDLSSRR` _allvideosettings_bdlss_rrenabled))
      (:`then_12`
        (if (> _allvideosettings_fsrmodeoptionid 0)
          (`|ExecutionSequence`
            (:`then_0`
              (switch `int` _allvideosettings_fsrmodeoptionid
                (:`0`
                  (`KismetSystemLibrary.ExecuteConsoleCommand` null "r.FidelityFX.FSR3.Enabled 0" null))
                (:`1`
                  (`KismetSystemLibrary.ExecuteConsoleCommand` null "r.FidelityFX.FSR3.Enabled 1" null :!label _label))
                (:`2`
                  (goto _label))
                (:`3`
                  (goto _label))
                (:`4`
                  (goto _label))))
            (:`then_1`
              (`KismetSystemLibrary.ExecuteConsoleCommand` null (`KismetStringLibrary.BuildString_Double` "" "r.FidelityFX.FSR3.QualityMode " (`KismetMathLibrary.Conv_IntToDouble` _allvideosettings_fsrmodeoptionid)) null)))))
      (:`then_13`
        (if _allvideosettings_bfsr3framegenenabled
          (`KismetSystemLibrary.ExecuteConsoleCommand` null "r.FidelityFX.FI.Enabled 1" null)
          (else
            (`KismetSystemLibrary.ExecuteConsoleCommand` null "r.FidelityFX.FI.Enabled 0" null))))
      (:`then_14`
        (`KismetSystemLibrary.ExecuteConsoleCommand` null (`KismetStringLibrary.BuildString_Double` "" "r.FidelityFX.FSR3.Sharpness " _allvideosettings_fsr3sharpness) null))
      (:`then_15`
        (if (> _allvideosettings_xessmodeoptionid 0)
          (switch `int` _allvideosettings_xessmodeoptionid
            (:`0`
              (`XeSSBlueprintLibrary.SetXeSSQualityMode` "Off"))
            (:`1`
              (`XeSSBlueprintLibrary.SetXeSSQualityMode` "UltraQuality"))
            (:`2`
              (`XeSSBlueprintLibrary.SetXeSSQualityMode` "Quality"))
            (:`3`
              (`XeSSBlueprintLibrary.SetXeSSQualityMode` "Balanced"))
            (:`4`
              (`XeSSBlueprintLibrary.SetXeSSQualityMode` "Performance")))))
      (:`then_16`
        (if (> _allvideosettings_nismodeoptionid 0)
          (switch `int` _allvideosettings_nismodeoptionid
            (:`0`
              (`NISLibrary.SetNISMode` "Off"))
            (:`1`
              (`NISLibrary.SetNISMode` "UltraQuality"))
            (:`2`
              (`NISLibrary.SetNISMode` "Quality"))
            (:`3`
              (`NISLibrary.SetNISMode` "Balanced"))
            (:`4`
              (`NISLibrary.SetNISMode` "Performance"))
            (:`5`
              (`NISLibrary.SetNISMode` "Custom")))))
      (:`then_17`
        (`NISLibrary.SetNISCustomScreenPercentage` _allvideosettings_niscustomscreenpercentage)))))

(fn `LoadSaveGame`
  (params (SaveSlotName :type String :default "OptionsSaveSlot0") (SaveUserID :type Integer))
  (returns (`AsBP Options Save Game` :type "/Game/CommonUI/Save/BP_OptionsSaveGame Object Reference") (SaveGameExist :type Boolean))
  (locals (`Save Slot Name` :type String :default "OptionsSaveSlot0") (`Save User Index` :type Integer))
  (set `local.Save Slot Name` SaveSlotName)
  (set `local.Save User Index` SaveUserID)
  (bind _returnvalue (`GameplayStatics.DoesSaveGameExist` (`local.Save Slot Name`) (`local.Save User Index`)))
  (if _returnvalue
    (bind _returnvalue_2 (`GameplayStatics.LoadGameFromSlot` (`local.Save Slot Name`) (`local.Save User Index`)))
    (bind _asbp_options_save_game (cast `/Game/CommonUI/Save/BP_OptionsSaveGame` _returnvalue_2))
    (return _asbp_options_save_game _returnvalue)
    (else
      (return null _returnvalue))))

(fn `PromptAction`
  (params (Condition :type Boolean) (PromptID :type Integer))
  (locals (PromptID :type Integer))
  (bind _returnvalue (`GameplayStatics.GetPlayerController` null))
  ;[0.05127 0.05127 0.05127] This will add a logic to the PromptID you added in the Button that shows the prompt.
  (switch `int` PromptID
    (:`0`
      (if Condition
        (`CommonInputSubsystem.SetCurrentInputType` (pcsubsystem `CommonInputSubsystem` _returnvalue) "MouseAndKeyboard")
        (`KismetSystemLibrary.QuitGame` null _returnvalue "Quit")
        (else
          (`KismetSystemLibrary.PrintString` null "BRUH"))))
    (:`1`
      (if Condition
        (bind _foundwidgets (`WidgetBlueprintLibrary.GetAllWidgetsOfClass` null "/Game/CommonUI/Foundation/Widgets/BPW_Container.BPW_Container_C" false))
        (for _array_element _foundwidgets
          (`CommonActivatableWidget.DeactivateWidget` _array_element)
          (`GameplayStatics.OpenLevelBySoftObjectPtr` null "/Game/CommonUI/Maps/LVL_Frontend.LVL_Frontend"))))))

(fn `ShowPrompt`
  (params (`Which Button` :type "/Game/CommonUI/Foundation/Buttons/BPW_GenericButton Object Reference"))
  (bind _foundwidgets (`WidgetBlueprintLibrary.GetAllWidgetsOfClass` null "/Game/CommonUI/Foundation/Widgets/BPW_Container.BPW_Container_C"))
  (for _array_element _foundwidgets
    _)
  (`/Game/CommonUI/Foundation/Widgets/BPW_Container.PushPrompt` _array_element (`/Game/CommonUI/Foundation/Buttons/BPW_GenericButton.PromptText` `Which Button`) (`/Game/CommonUI/Foundation/Buttons/BPW_GenericButton.PromptTitleText` `Which Button`) (`/Game/CommonUI/Foundation/Buttons/BPW_GenericButton.SetNoButtonText` `Which Button`) (`/Game/CommonUI/Foundation/Buttons/BPW_GenericButton.SetYesButtonText` `Which Button`) (`/Game/CommonUI/Foundation/Buttons/BPW_GenericButton.bShouldNoDeactivate` `Which Button`) (`/Game/CommonUI/Foundation/Buttons/BPW_GenericButton.bShouldYesDeactivate` `Which Button`) (`/Game/CommonUI/Foundation/Buttons/BPW_GenericButton.PromptID` `Which Button`)))