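; Parent player controller that sets up the game's UI container and serves as the entry point for prompt menus.
; On BeginPlay it creates and stores a BPW_Container widget, then applies post-process and video settings.
; ShowPrompt copies the calling button's prompt ID and Yes/No deactivation flags onto the controller, then pushes a prompt with that button's texts onto the container's stack.
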(event `self.ReceiveBeginPlay`
  ;[0 1 0.4375] On Begin Play, create the conatiner for all Widgets
  (bind _returnvalue (`|CreateWidget` "/Game/CommonUI/Foundation/Widgets/BPW_Container.BPW_Container_C"))
  (set `self.UIContainer` _returnvalue)
  ;[0.7109 1 0] Apply user settings
  (`/Game/CommonUI/BPFL_UI.ApplyPostProcessSettings`)
  (`/Game/CommonUI/BPFL_UI.ApplyVideoSettings`))

(fn `ShowPrompt`
  (params (WhichButton :type "/Game/CommonUI/Foundation/Buttons/BPW_GenericButton Object Reference"))
  ;[0.05127 0.05127 0.05127] We push the prompt menu on the stack and set the PromptID of the PlayerController with the value of the PromptID from the input button
  ;;[0.05127 0.05127 0.05127] We copy the value of the variables from the button to their respectives variable.
  (set `self.PromptID` (`/Game/CommonUI/Foundation/Buttons/BPW_GenericButton.PromptID` WhichButton))
  (set `self.bShouldNoDeactivate` (`/Game/CommonUI/Foundation/Buttons/BPW_GenericButton.bShouldNoDeactivate` WhichButton))
  (set `self.bShouldYesDeactivate` (`/Game/CommonUI/Foundation/Buttons/BPW_GenericButton.bShouldYesDeactivate` WhichButton))
  (`/Game/CommonUI/Foundation/Widgets/BPW_Container.PushPrompt` (`self.UIContainer`) (`/Game/CommonUI/Foundation/Buttons/BPW_GenericButton.PromptText` WhichButton) (`/Game/CommonUI/Foundation/Buttons/BPW_GenericButton.PromptTitleText` WhichButton) (`/Game/CommonUI/Foundation/Buttons/BPW_GenericButton.SetNoButtonText` WhichButton) (`/Game/CommonUI/Foundation/Buttons/BPW_GenericButton.SetYesButtonText` WhichButton) false false 0))

(fn `UserConstructionScript`)